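; CS_ReefBP is a damageable reef actor that destroys itself when its health runs out.
; AnyDamage subtracts damage from CurrentHealth, prints the remaining value and destroys the actor at zero or below.
; Plane hits from Projectile_BP jump into that same chain, reusing the AnyDamage event's Damage pin rather than supplying their own amount.
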(event OnComponentHit(Plane)
  (params (HitComponent :type Primitive%20Component%20Object%20Reference) (OtherActor :type Actor%20Object%20Reference) (OtherComp :type Primitive%20Component%20Object%20Reference) (NormalImpulse :type Vector :default "0, 0, 0") (Hit :type Hit%20Result%20Structure%20%28by%20ref%29))
  ;[1 0.3265 0.895] Damage towards reef - Hayden
  (if (== OtherActor "/Game/CS_Blueprints/CS_Enemy/Projectile_BP.Projectile_BP")
    (Variables|Default|SetCurrentHealth (- (Variables|Default|GetCurrentHealth) (stale Game|Damage|EventAnyDamage Damage)))
    (Development|PrintString (Utilities|String|ToString(Integer) (Variables|Default|GetCurrentHealth)))
    (if (<= (Variables|Default|GetCurrentHealth) 0)
      (Actor|DestroyActor self))))

(event EventBeginPlay)

(event Collision|EventActorBeginOverlap
  (params (OtherActor :type Actor%20Object%20Reference)))

(event EventTick
  (params (DeltaSeconds :type Float%20%28single-precision%29))
  ;[1 0.3265 0.895] Damage towards reef - Hayden
)

(event Game|Damage|EventAnyDamage
  (params (Damage :type Float%20%28single-precision%29) (DamageType :type Damage%20Type%20Object%20Reference) (InstigatedBy :type Controller%20Object%20Reference) (DamageCauser :type Actor%20Object%20Reference))
  ;[1 0.3265 0.895] Damage towards reef - Hayden
  (Variables|Default|SetCurrentHealth (- (Variables|Default|GetCurrentHealth) Damage))
  (Development|PrintString (Utilities|String|ToString(Integer) (Variables|Default|GetCurrentHealth)))
  (if (<= (Variables|Default|GetCurrentHealth) 0)
    (Actor|DestroyActor self)))

(fn ConstructionScript)