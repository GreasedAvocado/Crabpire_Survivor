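; Player Blueprint that handles movement, XP leveling and health for the player character.
; BeginPlay adds the Enhanced Input mapping context, and IA_Move feeds movement input.
; PickupTrigger overlaps consume trash XP or health pickups: XP reaching the threshold triggers LevelUp, which only scales the next threshold without resetting XP.
; Damage lowers health and re-enables healing until max health is reached, while death only prints a message.
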(event OnComponentBeginOverlap(PickupTrigger)
  (params (OverlappedComponent :type Primitive%20Component%20Object%20Reference) (OtherActor :type Actor%20Object%20Reference) (OtherComp :type Primitive%20Component%20Object%20Reference) (OtherBodyIndex :type Integer) (bFromSweep :type Boolean) (SweepResult :type Hit%20Result%20Structure%20%28by%20ref%29))
  (bind _astrash_xp_bp (Utilities|Casting|CastToTrashXP_BP OtherActor)
    (:then
      (bind _output_get (Variables|Default|SetAs%20Trash%20XP%20BP _astrash_xp_bp))
      (CallFunction|GainXP)
      (Actor|DestroyActor _output_get))
    (:CastFailed
      (bind _ashealth_pick_up_bp (Utilities|Casting|CastToHealthPickUp_BP OtherActor))
      (bind _output_get_2 (Variables|Default|SetAs%20Health%20Pick%20Up%20BP _ashealth_pick_up_bp))
      (CallFunction|GainHealth)
      (Actor|DestroyActor _output_get_2))))

(event Custom|GainXP
  ;[1 1 1] Gain xp - Adam
  (bind _output_get (Variables|Default|SetXPCurrent (+ (Variables|Default|GetXPCurrent) (Variables|Default|GetXPGained))))
  (Development|PrintString (Utilities|String|ToString(Float) _output_get))
  (if (>= _output_get (Variables|Default|GetXPTotal))
    (CallFunction|LevelUp)
    (Development|PrintString "Level Up!")))

(event Custom|LevelUp
  ;[1 1 1] Add Upgrade menu to level up event - Adam
  (bind _output_get (Variables|Default|SetXPTotal (* (Variables|Default|GetXPTotal) 1.2)))
  (Development|PrintString (Utilities|String|ToString(Float) _output_get)))

(event Input|EnhancedActionEvents|EnhancedInputActionIA_Move
  (params (ActionValue :type Vector%202D%20Structure) (ElapsedSeconds :type Float%20%28double-precision%29) (TriggeredSeconds :type Float%20%28double-precision%29) (InputAction :type Input%20Action%20Object%20Reference :default "/Game/CS_Blueprints/CS_Inputs/CS_InputActions/IA_Move.IA_Move"))
  (:Triggered
    (Pawn|Input|AddMovementInput (Math|Vector|GetRightVector (Math|Rotator|MakeRotator (.x ActionValue) 0.0 0.0)) (.x ActionValue) false)
    (Pawn|Input|AddMovementInput (Math|Vector|GetForwardVector (Math|Rotator|MakeRotator 0.0 (.y ActionValue) 0.0)) (.y ActionValue) false)))

(event EventBeginPlay
  (bind _returnvalue (PlayerController|LocalPlayerSubsystems|GetEnhancedInputLocalPlayerSubsystem))
  (Utilities|IsValid _returnvalue
    (:Is%20Valid
      (Input|AddMappingContext _returnvalue "/Game/CS_Blueprints/CS_Inputs/CS_InputMappingContext.CS_InputMappingContext" 0 "(bIgnoreAllPressedKeysUntilRelease=True,bForceImmediately=False)"))))

(event Collision|EventActorBeginOverlap
  (params (OtherActor :type Actor%20Object%20Reference)))

(event EventTick
  (params (DeltaSeconds :type Float%20%28single-precision%29)))

(event Game|Damage|EventAnyDamage
  (params (Damage :type Float%20%28single-precision%29) (DamageType :type Damage%20Type%20Object%20Reference) (InstigatedBy :type Controller%20Object%20Reference) (DamageCauser :type Actor%20Object%20Reference))
  ;[1 1 1] Player Take Damage - Adam
  (bind _output_get (Variables|Default|SetHealth (- (Variables|Default|GetHealth) Damage)))
  (Development|PrintString (Utilities|String|ToString(Float) _output_get))
  (Variables|Default|SetbCanGainHealth? true)
  (if (<= (Variables|Default|GetHealth) 0.0)
    (Development|PrintString "You Died")))

(fn ConstructionScript)

(fn GainHealth
  (if (Variables|Default|GetbCanGainHealth?)
    (bind _output_get (Variables|Default|SetHealth (+ (Variables|Default|GetHealth) 1.0)))
    (Development|PrintString (Utilities|String|ToString(Float) _output_get))
    (if (>= (Variables|Default|GetHealth) (Variables|Default|GetHealthMax))
      (Variables|Default|SetbCanGainHealth? false)
      (return))))