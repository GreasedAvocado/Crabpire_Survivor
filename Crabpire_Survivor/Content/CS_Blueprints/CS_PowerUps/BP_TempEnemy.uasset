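; BP_TempEnemy is a temporary enemy actor in the power-ups folder, with all of its behavior currently disconnected.
; A custom event pushes its Cube along negative X with a velocity-change impulse, but the looping timer meant to fire it never runs.
; TakeDamage is an empty entry, as its unwired logic for reducing Health, printing it and destroying the actor at zero never executes.
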(event Custom|CustomEvent
  (Physics|AddImpulse (Variables|Default|GetCube) "-200.000000,0.000000,0.000000" "None" true))

(event EventBeginPlay)

(event Collision|EventActorBeginOverlap
  (params (OtherActor :type Actor%20Object%20Reference)))

(event EventTick
  (params (DeltaSeconds :type Float%20%28single-precision%29)))

(fn ConstructionScript)

(fn TakeDamage
  (params (Damage :type Float%20%28double-precision%29)))