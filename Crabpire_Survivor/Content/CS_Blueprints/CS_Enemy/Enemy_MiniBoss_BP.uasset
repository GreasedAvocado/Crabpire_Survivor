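; Mini-boss enemy that advances on the reef until it sees the player, then permanently switches to chasing them.
; AI MoveTo closes in and caches the target's location, then a delayed line-trace shot repeats, resuming the chase when the player moves.
; A timeline squashes its plane during pursuit, while Tick rotates the capsule toward its target.
; Damage reduces health, and death randomly drops trash XP or a health pickup.
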(event OnSeePawn(PawnSensing)
  (params (Pawn :type Pawn%20Object%20Reference))
  (Variables|Default|SetHasSeenPlayer true)
  (CallFunction|ChaseTarget))

(event Custom|Shoot
  (if (Variables|Default|GetHasSeenPlayer)
    (bind _isplayerstill (CallFunction|IsPlayerStandingStill))
    (if _isplayerstill
      (Utilities|FlowControl|Delay 0.4 :!label _label)
      (bind _outhit (Collision|LineTraceByChannel (Transformation|GetWorldLocation (Variables|Character|GetMesh)) (Variables|Default|GetLastLocation) "TraceTypeQuery1" false 0 "ForDuration"))
      (Game|Damage|ApplyDamage (.hitactor _outhit) 1.0 0 0)
      (CallFunction|Shoot)
      (else
        (CallFunction|ChaseTarget)))
    (else
      (goto _label))))

(event Custom|Chase%20Target
  (bind _returnvalue (Game|GetPlayerCharacter 0))
  (bind _reef (Variables|Default|GetReef))
  (if (Variables|Default|GetHasSeenPlayer)
    (Utilities|FlowControl|Sequence
      (:then_0
        (AI|AIMoveTo self "0, 0, 0" _returnvalue 2e+02 false
          (:OnSuccess
            (Variables|Default|SetLastLocation (Transformation|GetWorldLocation (Variables|/Script/Engine.Character|GetMesh _returnvalue)))
            (CallFunction|Shoot))
          (:OnFail
            (CallFunction|ChaseTarget))))
      (:then_1
        (bind _alpha (Timeline|Enemy3%20Bobbing PlayFromStart)
          (:Update
            (Transformation|SetRelativeScale3D (Variables|Default|GetPlane) (Math|Vector|Lerp(Vector) (Variables|Default|GetRelative%20Scale%203D) (* (Variables|Default|GetRelative%20Scale%203D) (Variables|Default|GetWalkingSqueezeVector)) _alpha))))))
    (else
      (Utilities|FlowControl|Sequence
        (:then_0
          (AI|AIMoveTo self "0, 0, 0" _reef 2e+02 false
            (:OnSuccess
              (Variables|Default|SetLastLocation (Transformation|GetWorldLocation (Variables|/Script/Engine.Actor|GetRootComponent _reef)))
              (CallFunction|Shoot))
            (:OnFail
              (CallFunction|ChaseTarget))))
        (:then_1
          (Timeline|Enemy3%20Bobbing PlayFromStart))))))

(event EventBeginPlay
  (Utilities|FlowControl|Sequence
    (:then_0
      (bind _returnvalue (Actor|GetActorOfClass "/Game/CS_Blueprints/CS_ReefBP/CS_ReefBP.CS_ReefBP_C"))
      (Variables|Default|SetReef _returnvalue)
      (Utilities|FlowControl|Delay 2.0)
      (CallFunction|ChaseTarget))
    (:then_1
      (Variables|Default|SetRelative%20Scale%203D (Variables|/Script/Engine.SceneComponent|GetRelativeScale3D (Variables|Default|GetPlane))))))

(event Game|Damage|EventAnyDamage
  (params (Damage :type Float%20%28single-precision%29) (DamageType :type Damage%20Type%20Object%20Reference) (InstigatedBy :type Controller%20Object%20Reference) (DamageCauser :type Actor%20Object%20Reference))
  (bind _output_get (Variables|Default|SetHealth (Math|Float|Truncate (- (Variables|Default|GetHealth) Damage))))
  (if (<= _output_get 0)
    (CallFunction|LootDrop)
    (Actor|DestroyActor)))

(event EventTick
  (params (DeltaSeconds :type Float%20%28single-precision%29))
  (if (Variables|Default|GetHasSeenPlayer)
    (bind _isplayerstill (CallFunction|IsPlayerStandingStill))
    (if (not _isplayerstill)
      (CallFunction|LookatPlayer))
    (else
      (Transformation|SetWorldRotation (Variables|Collision|GetCapsuleComponent) (Math|Rotator|FindLookatRotation (Transformation|GetWorldLocation (Variables|Character|GetMesh)) (Transformation|GetWorldLocation (Variables|/Game/CS_Blueprints/CS_ReefBP/CS_ReefBP.CS_ReefBP_C|GetPlane (Variables|Default|GetReef)))) false false))))

(fn ConstructionScript)

(fn IsPlayerStandingStill
  (return (Utilities|Operators|EqualEqual (Variables|Default|GetLastLocation) (Transformation|GetWorldLocation (Variables|/Script/Engine.Character|GetMesh (Game|GetPlayerCharacter 0))) 0.0)))

(fn LookatPlayer
  (Transformation|SetWorldRotation (Variables|Collision|GetCapsuleComponent) (Math|Rotator|FindLookatRotation (Transformation|GetWorldLocation (Variables|Collision|GetCapsuleComponent)) (Class|PlayerController|GetFocalLocation (Game|GetPlayerController 0))) false false))

(fn LookatReef)

(fn LootDrop
  (bind _mesh (Variables|Character|GetMesh))
  (bind _returnvalue (Transformation|GetWorldLocation _mesh))
  (if (== (.OutItem (Utilities|Array|Random (Variables|Default|GetXPLiklyness))) 1)
    (Game|SpawnActorfromClass "/Game/CS_Blueprints/CS_Enemy/TrashXP_BP.TrashXP_BP_C" (Math|Transform|MakeTransform (Transformation|GetWorldLocation (Variables|Character|GetMesh)) "0, 0, 0" "1.000000,1.000000,1.000000") "AdjustIfPossibleButAlwaysSpawn" "MultiplyWithRoot" 0 0)
    (elif (== (.OutItem (Utilities|Array|Random (Variables|Default|GetHealth%20Liklyness))) 5)
      (Game|SpawnActorfromClass "/Game/CS_Blueprints/CS_Enemy/HealthPickUp_BP.HealthPickUp_BP_C" (Math|Transform|MakeTransform (Math|Vector|MakeVector (.x _returnvalue) (.y _returnvalue) (.z _returnvalue)) "0, 0, 0" "1.000000,1.000000,1.000000") "AdjustIfPossibleButAlwaysSpawn" "MultiplyWithRoot" 0 0))))