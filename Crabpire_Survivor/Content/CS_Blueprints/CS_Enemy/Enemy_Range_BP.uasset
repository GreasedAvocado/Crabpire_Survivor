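; Ranged enemy that advances on the reef and fires projectiles at it, switching permanently to the player once PawnSensing spots a pawn.
; AIMoveTo retries until in range, then a self-calling Shoot loop spawns a delayed projectile, resuming the chase whenever the player leaves the saved location.
; Tick turns the capsule toward the reef, or toward the player controller's focal point while the player moves.
; Damage reduces Health and destroys the actor at zero.
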(event OnSeePawn(PawnSensing)
  (params (Pawn :type Pawn%20Object%20Reference))
  (Variables|Default|SetHasSeenPlayer true)
  (CallFunction|ChaseTarget))

(event Custom|Shoot
  (if (Variables|Default|GetHasSeenPlayer)
    (bind _isplayerstill (CallFunction|IsPlayerStandingStill))
    (if _isplayerstill
      (Utilities|FlowControl|Delay 1.0 :!label _label)
      (Game|SpawnActorfromClass "/Game/CS_Blueprints/CS_Enemy/Projectile_BP.Projectile_BP_C" (Transformation|GetWorldTransform (Variables|Default|GetSpawnProjectile)) "Undefined" "MultiplyWithRoot" 0 0)
      (CallFunction|Shoot)
      (else
        (CallFunction|ChaseTarget)))
    (else
      (goto _label))))

(event Custom|Chase%20Target
  (bind _returnvalue (Game|GetPlayerCharacter 0))
  (bind _reef (Variables|Default|GetReef))
  (if (Variables|Default|GetHasSeenPlayer)
    (AI|AIMoveTo self "0, 0, 0" _returnvalue 5e+02 false
      (:OnSuccess
        (Variables|Default|SetLastLocation (Transformation|GetWorldLocation (Variables|/Script/Engine.Character|GetMesh _returnvalue)))
        (CallFunction|Shoot))
      (:OnFail
        (CallFunction|ChaseTarget)))
    (else
      (AI|AIMoveTo self "0, 0, 0" _reef 5e+02 false
        (:OnSuccess
          (Variables|Default|SetLastLocation (Transformation|GetWorldLocation (Variables|/Script/Engine.Actor|GetRootComponent _reef)))
          (CallFunction|Shoot))
        (:OnFail
          (CallFunction|ChaseTarget))))))

(event EventBeginPlay
  (bind _returnvalue (Actor|GetActorOfClass "/Game/CS_Blueprints/CS_ReefBP/CS_ReefBP.CS_ReefBP_C"))
  (Variables|Default|SetReef _returnvalue)
  (Utilities|FlowControl|Delay 2.0)
  (CallFunction|ChaseTarget))

(event Game|Damage|EventAnyDamage
  (params (Damage :type Float%20%28single-precision%29) (DamageType :type Damage%20Type%20Object%20Reference) (InstigatedBy :type Controller%20Object%20Reference) (DamageCauser :type Actor%20Object%20Reference))
  (bind _output_get (Variables|Default|SetHealth (Math|Float|Truncate (- (Variables|Default|GetHealth) Damage))))
  (if (<= _output_get 0)
    (Actor|DestroyActor)))

(event Collision|EventActorBeginOverlap
  (params (OtherActor :type Actor%20Object%20Reference))
  (Development|PrintString (Utilities|GetDisplayName OtherActor)))

(event EventTick
  (params (DeltaSeconds :type Float%20%28single-precision%29))
  (if (Variables|Default|GetHasSeenPlayer)
    (bind _isplayerstill (CallFunction|IsPlayerStandingStill))
    (if (not _isplayerstill)
      (CallFunction|LookatPlayer))
    (else
      (Transformation|SetWorldRotation (Variables|Collision|GetCapsuleComponent) (Math|Rotator|FindLookatRotation (Transformation|GetWorldLocation (Variables|Character|GetMesh)) (Transformation|GetWorldLocation (Variables|/Game/CS_Blueprints/CS_ReefBP/CS_ReefBP.CS_ReefBP_C|GetPlane (Variables|Default|GetReef)))) false false))))

(fn ConstructionScript)

(fn IsPlayerStandingStill
  (return (Utilities|Operators|EqualEqual (Variables|Default|GetLastLocation) (Transformation|GetWorldLocation (Variables|/Script/Engine.Character|GetMesh (Game|GetPlayerCharacter 0))) 0.0)))

(fn LookatPlayer
  (Transformation|SetWorldRotation (Variables|Collision|GetCapsuleComponent) (Math|Rotator|FindLookatRotation (Transformation|GetWorldLocation (Variables|Collision|GetCapsuleComponent)) (Class|PlayerController|GetFocalLocation (Game|GetPlayerController 0))) false false))

(fn LookatReef)