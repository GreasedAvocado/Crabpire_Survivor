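; Enemy spawner actor that continuously spawns AI enemies inside a box volume, starting at BeginPlay.
; Each cycle picks either a ranged or a chasing enemy at random and places it at a random point within the SpawnRadius box, ignoring collision.
; The spawn event then waits for the CoolDown delay and calls itself, looping with no spawn cap or stop condition.
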(event Custom|Spawn%20Enemy
  (bind _spawn_radius (Variables|Default|GetSpawn%20Radius))
  (bind _returnvalue (Transformation|GetWorldLocation _spawn_radius))
  (bind _returnvalue_2 (Components|Box|GetScaledBoxExtent _spawn_radius))
  (bind _returnvalue_3 (Math|Random|RandomPointinBoundingBox _returnvalue _returnvalue_2))
  (if (Math|Random|RandomBool)
    (AI|SpawnAIFromClass "/Game/CS_Blueprints/CS_Enemy/Enemy_Range_BP.Enemy_Range_BP_C" 0 _returnvalue_3 "0, 0, 0" true 0)
    (else
      (AI|SpawnAIFromClass "/Game/CS_Blueprints/CS_Enemy/Enemy_Chase_BP.Enemy_Chase_BP_C" 0 _returnvalue_3 "0, 0, 0" true 0)))
  (Utilities|FlowControl|Delay (Variables|Default|GetCoolDown))
  (CallFunction|SpawnEnemy))

(event EventBeginPlay
  (CallFunction|SpawnEnemy))

(event Collision|EventActorBeginOverlap
  (params (OtherActor :type Actor%20Object%20Reference)))

(event EventTick
  (params (DeltaSeconds :type Float%20%28single-precision%29)))

(fn ConstructionScript)