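; Chasing enemy that damages player-tagged components on hit, destroying itself in the process.
; After a startup delay it moves to a hardcoded point, switching to follow the player once PawnSensing sees a pawn, and retries failed moves.
; Incoming damage lowers Health; death rolls random arrays to drop TrashXP_BP or, failing that, possibly HealthPickUp_BP.
; The CS_ReefBP reference is cached but unused.
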(event OnSeePawn(PawnSensing)
  (params (Pawn :type Pawn%20Object%20Reference))
  (Variables|Default|SetHasSeenPlayer true)
  (CallFunction|ChasePlayer))

(event Custom|Chase%20Player
  (if (Variables|Default|GetHasSeenPlayer)
    (AI|AIMoveTo self "0, 0, 0" (Game|GetPlayerCharacter 0) 0.0 false
      (:OnFail
        (CallFunction|ChasePlayer)))
    (else
      (AI|AIMoveTo self "1440.000000,1640.000000,5.000000" 0 0.0 false
        (:OnFail
          (CallFunction|ChasePlayer))))))

(event EventBeginPlay
  (Utilities|FlowControl|Delay 2.0)
  (bind _returnvalue (Actor|GetActorOfClass "/Game/CS_Blueprints/CS_ReefBP/CS_ReefBP.CS_ReefBP_C"))
  (Variables|Default|SetReef _returnvalue)
  (CallFunction|ChasePlayer))

(event Game|Damage|EventAnyDamage
  (params (Damage :type Float%20%28single-precision%29) (DamageType :type Damage%20Type%20Object%20Reference) (InstigatedBy :type Controller%20Object%20Reference) (DamageCauser :type Actor%20Object%20Reference))
  (bind _output_get (Variables|Default|SetHealth (Math|Float|Truncate (- (Variables|Default|GetHealth) Damage))))
  (if (<= _output_get 0)
    (CallFunction|LootDrop)
    (Actor|DestroyActor)))

(event Collision|EventHit
  (params (MyComp :type Primitive%20Component%20Object%20Reference) (Other :type Actor%20Object%20Reference) (OtherComp :type Primitive%20Component%20Object%20Reference) (bSelfMoved :type Boolean) (HitLocation :type Vector :default "0, 0, 0") (HitNormal :type Vector :default "0, 0, 0") (NormalImpulse :type Vector :default "0, 0, 0") (Hit :type Hit%20Result%20Structure%20%28by%20ref%29))
  (if (Components|ComponentHasTag OtherComp "Player")
    (if true
      (Game|Damage|ApplyDamage Other 1.0 0 0)
      (Actor|DestroyActor))))

(fn ConstructionScript)

(fn LootDrop
  (bind _mesh (Variables|Character|GetMesh))
  (bind _returnvalue (Transformation|GetWorldLocation _mesh))
  (if (== (.OutItem (Utilities|Array|Random (Variables|Default|GetXPLiklyness))) 1)
    (Game|SpawnActorfromClass "/Game/CS_Blueprints/CS_Enemy/TrashXP_BP.TrashXP_BP_C" (Math|Transform|MakeTransform (Transformation|GetWorldLocation (Variables|Character|GetMesh)) "0, 0, 0" "1.000000,1.000000,1.000000") "AdjustIfPossibleButAlwaysSpawn" "MultiplyWithRoot" 0 0)
    (elif (== (.OutItem (Utilities|Array|Random (Variables|Default|GetHealthLiklyness))) 5)
      (Game|SpawnActorfromClass "/Game/CS_Blueprints/CS_Enemy/HealthPickUp_BP.HealthPickUp_BP_C" (Math|Transform|MakeTransform (Math|Vector|MakeVector (.x _returnvalue) (.y _returnvalue) (.z _returnvalue)) "0, 0, 0" "1.000000,1.000000,1.000000") "Undefined" "MultiplyWithRoot" 0 0))))